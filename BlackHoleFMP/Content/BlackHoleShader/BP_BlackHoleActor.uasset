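; Black hole actor that feeds a shader parameter collection and keeps its point light matched to the shared colour.
; The construction script sets the Niagara asteroid field's outer disk radius and writes the BlackHoleEnv world location into MPCBH as BlackHolePosition.
; It also colours the light from MPCBH's LightColour and starts a looping timer that calls RegenerateLighting to reapply that colour every second.
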(event `self.ReceiveBeginPlay`)

(event `RegenerateLighting`
  (bind _returnvalue (`KismetMaterialLibrary.GetVectorParameterValue` (`self.MPC_BH`) "LightColour"))
  (`LightComponent.SetLightColor` (`self.PointLight`) _returnvalue true))

(fn `UserConstructionScript`
  (bind _mpc_bh (`self.MPC_BH`))
  (`NiagaraComponent.SetVariableFloat` (`self.AsteroidField`) "User.DiskOuterRadius" (* 200.0 120.0))
  (`KismetMaterialLibrary.SetVectorParameterValue` _mpc_bh "BlackHolePosition" (`KismetMathLibrary.Conv_VectorToLinearColor` (`SceneComponent.K2_GetComponentLocation` (`self.BlackHoleEnv`))))
  (`KismetMaterialLibrary.GetVectorParameterValue` _mpc_bh "BlackHolePosition")
  (bind _returnvalue (`KismetMaterialLibrary.GetVectorParameterValue` _mpc_bh "LightColour"))
  (`LightComponent.SetLightColor` (`self.PointLight`) _returnvalue true)
  (`KismetSystemLibrary.K2_SetTimer` null "RegenerateLighting" 1.0 true))